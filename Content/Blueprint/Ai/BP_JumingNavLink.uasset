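; Smart nav link actor that makes Characters jump to the link's destination when they reach it.
; SmartLinkReached launches the Character with a velocity CalculateVelocity derives from start, destination and JumpDuration, added to its current velocity.
; CalculateVelocity solves a ballistic arc with hard-coded gravity, but its Y component is inverted: duration divided by distance, unlike X.
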(event `self.ReceiveSmartLinkReached`
  (params (Agent :type "Actor Object Reference") (Destination :type "Vector Structure (by ref)"))
  (bind _ascharacter (cast `Character` Agent))
  (bind _velcoty (`self.CalculateVelocity` Destination (`self.K2_GetActorLocation` _ascharacter) (`self.JumpDuration`)))
  (`Character.LaunchCharacter` _ascharacter _velcoty false false))

(fn `CalculateVelocity`
  (params (Dest :type "Vector Structure") (Start :type "Vector Structure") (Durationj :type "Float (double-precision)"))
  (returns (Velcoty :type "Vector Structure"))
  (locals (InDuration :type "Float (double-precision)"))
  (bind _induration (`local.InDuration`))
  (set `local.InDuration` Durationj)
  (return (`KismetMathLibrary.MakeVector` (/ (- (.x Dest) (.x Start)) _induration) (/ _induration (- (.y Dest) (.y Start))) (/ (- (.z Dest) (+ (.z Start) (* (`KismetMathLibrary.Square` (`local.InDuration`)) -0.5 982.0))) _induration))))

(fn `UserConstructionScript`)