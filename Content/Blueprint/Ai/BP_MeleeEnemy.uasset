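; BP_MeleeEnemy is a melee enemy Blueprint, a child class that extends a parent's Attack behavior.
; Incoming damage reduces Health, and at zero or below the enemy prints a defeat message and destroys itself.
; Attack calls the parent version and then prints the enemy's name as attacking, while SetMaterial applies a given material to the mesh's first slot.
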(event `self.ReceiveAnyDamage`
  (params (Damage :type "Float (single-precision)") (DamageType :type "DamageType Object Reference") (InstigatedBy :type "Controller Object Reference") (DamageCauser :type "Actor Object Reference"))
  (bind _output_get (set `self.Health` (- (`self.Health`) Damage)))
  (if (<= _output_get 0.0)
    (`KismetSystemLibrary.PrintString` "Enemy Defeated")
    (`self.K2_DestroyActor`)))

(fn `Attack`
  (params (Target :type "Vector Structure"))
  (`parent.Attack` Target)
  (`KismetSystemLibrary.PrintString` (`KismetStringLibrary.Concat_StrStr` (`KismetSystemLibrary.GetDisplayName` self) " attacks")))

(fn `SetMaterial`
  (params (Material :type "Material Object Reference"))
  (`PrimitiveComponent.SetMaterial` (`self.Mesh`) 0 Material))

(fn `UserConstructionScript`
  (`parent.UserConstructionScript`))